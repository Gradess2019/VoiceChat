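; Free-flying test pawn for networked voice chat, with camera-relative movement, mouse look and a V key toggle for voice capture.
; On begin play, a local client requests the game mode's public IP through server and client events, retrying short results, and stores it on the Voice component.
; A locally controlled server instead opens a hardcoded address.
; Tick prints address and capture stats; L forces garbage collection.
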(event Custom|GetPublicIP_Client
  (params (IP :type String))
  (bind _output_get (Variables|/Script/VoiceChat.VoiceComponent|SetAddress (Variables|Default|GetVoice) IP))
  (if (< (Utilities|String|Len _output_get) 8)
    (Development|PrintString "Addr is empty! Retrying...")
    (Utilities|FlowControl|Delay 0.2)
    (CallFunction|GetPublicIPServer)))

(event Custom|GetPublicIP_Server
  (bind _publicip (Class|BPIVoiceServerGameMode|GetPublicIP(Message) (Game|GetGameMode)))
  (CallFunction|GetPublicIPClient _publicip))

(event EventBeginPlay
  (if (Pawn|IsLocallyControlled)
    (Class|VOIPStatics|SetMicThreshold 0.005)
    (Development|ExecuteConsoleCommand "r.VSync 1" 0)
    (if (Networking|IsServer)
      (Development|ExecuteConsoleCommand (Utilities|String|Append "open " "91.76.97.152:7777") 0)
      (else
        (CallFunction|GetPublicIPServer)))))

(event EventTick
  (params (DeltaSeconds :type Float%20%28single-precision%29))
  (bind _voice (Variables|Default|GetVoice))
  (Utilities|IsValid 0
    (:Is%20Valid
      (Development|PrintString (Variables|/Script/VoiceChat.VoiceComponent|GetAddress (Variables|Default|GetVoice)) true false "(R=0.000000,G=0.660000,B=1.000000,A=1.000000)" 0.0))
    (:Is%20Not%20Valid
      _))
  (Utilities|IsValid (Variables|Default|GetVoice)
    (:Is%20Valid
      (if (Pawn|IsLocallyControlled)
        (Development|PrintText (Utilities|Text|FormatText "Volume: {0} 
Capturing: {1} 
Total bytes: {2}" (Variables|/Script/VoiceChat.VoiceComponent|GetVoiceCaptureVolume _voice) (Utilities|Text|ToText(Boolean) (Class|VoiceComponent|IsCapturing _voice)) (Utilities|Text|ToText(String) (Variables|/Script/VoiceChat.VoiceComponent|GetNumOfBytes _voice))) true false "(R=0.000000,G=0.660000,B=1.000000,A=1.000000)" 0.0)))))

(event Input|AxisEvents|InputAxisMoveRight
  (params (AxisValue :type Float%20%28single-precision%29))
  (Pawn|Input|AddMovementInput (Math|Vector|GetRightVector (Variables|Default|GetCamera)) AxisValue false))

(event Input|AxisEvents|InputAxisLookUp
  (params (AxisValue :type Float%20%28single-precision%29))
  (Pawn|Input|AddControllerPitchInput AxisValue))

(event Input|AxisEvents|InputAxisTurnAround
  (params (AxisValue :type Float%20%28single-precision%29))
  (Pawn|Input|AddControllerYawInput AxisValue))

(event Input|AxisEvents|InputAxisMoveForward
  (params (AxisValue :type Float%20%28single-precision%29))
  (Pawn|Input|AddMovementInput (Math|Vector|GetForwardVector (Variables|Default|GetCamera)) AxisValue false))

(event Input|KeyboardEvents|L
  (params (Key :type Key%20Structure :default "None"))
  (:Pressed
    (Utilities|Platform|CollectGarbage)
    (Development|PrintString "COLLECTED")))

(event Input|KeyboardEvents|V
  (params (Key :type Key%20Structure :default "None"))
  (bind _voice (Variables|Default|GetVoice))
  (:Pressed
    (Utilities|FlowControl|FlipFlop
      (:A
        (Class|VoiceComponent|Start _voice))
      (:B
        (Class|VoiceComponent|Stop _voice)))))

(fn ConstructionScript)