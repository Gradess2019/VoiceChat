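; BP_VoiceGameMode is a game mode that hosts a voice server on dedicated servers.
; On BeginPlay, if running as a dedicated server, it constructs a VoiceServer object owned by itself, stores it and initializes it.
; GetPublicIP returns that object's public IP, or an empty string when no valid voice server exists.
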(event EventBeginPlay
  (if (Networking|IsDedicatedServer)
    (CallFunction|InitVoiceServer)))

(fn ConstructionScript)

(fn InitVoiceServer
  (bind _returnvalue (Game|ConstructObjectfromClass "/Script/VoiceChat.VoiceServer" self))
  (bind _output_get (Variables|Default|SetVoiceServer _returnvalue))
  (Class|VoiceServer|Init _output_get))

(fn GetPublicIP
  (bind _voiceserver (Variables|Default|GetVoiceServer))
  (Utilities|IsValid _voiceserver
    (:Is%20Valid
      (return (Variables|/Script/VoiceChat.VoiceServer|GetPublicIP _voiceserver)))
    (:Is%20Not%20Valid
      (return ""))))